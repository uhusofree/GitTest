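; Game state Blueprint that tracks the score and ends the game when it is won.
; AddScore adds points, compares the total with BP_GameMode's ScoreToWin, calls WinState once reached, and returns the score.
; WinState shows a WBP_EndState widget, then quits the game after a short delay.
; LoseState is an empty stub, and Tick prints the score every frame.
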(event `self.ReceiveTick`
  (params (DeltaSeconds :type "Float (single-precision)"))
  (`KismetSystemLibrary.PrintString` (`KismetStringLibrary.Conv_IntToString` (`self.Score`)) true true (struct :`G` 0.66 :`B` 1.0 :`A` 1.0) DeltaSeconds))

(event `WinState`
  (bind _returnvalue (`|CreateWidget` "/Game/MIscellaneous/WBP_EndState.WBP_EndState_C"))
  (set `/Game/MIscellaneous/WBP_EndState.EndState` "NewEnumerator1" _returnvalue)
  (`UserWidget.AddToViewport` _returnvalue 0)
  (`KismetSystemLibrary.Delay` 2.0)
  (`KismetSystemLibrary.QuitGame` null "Quit"))

(event `LoseState`)

(fn `AddScore`
  (params (PointsToAdd :type Integer :default 1))
  (returns (Score :type Integer))
  (set `self.Score` (+ PointsToAdd (`self.Score`)))
  (bind _asbp_game_mode (cast `/Game/MIscellaneous/BP_GameMode` (`GameplayStatics.GetGameMode`))
    (:`then`
      (if (>= (`self.Score`) (`/Game/MIscellaneous/BP_GameMode.ScoreToWin` _asbp_game_mode))
        (`self.WinState`)
        (return (`self.Score`))
        (else
          (return (`self.Score`)))))
    (:`CastFailed`
      (return (`self.Score`)))))

(fn `UserConstructionScript`)