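; BP_DoorFrame is a door that swings between rotation states when interaction interface events start or stop.
; A timeline lerps the door mesh between rotations mapped to each state, and the construction script applies the initial state's rotation.
; Requests arriving mid-transition are queued and replayed on completion.
; Box-overlap logic for player-triggered, side-dependent opening is disconnected, so StartInteract always requests the same open state.
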(event `self.Box.OnComponentBeginOverlap`
  (params (OverlappedComponent :type "PrimitiveComponent Object Reference") (OtherActor :type "Actor Object Reference") (OtherComp :type "PrimitiveComponent Object Reference") (OtherBodyIndex :type Integer) (bFromSweep :type Boolean) (SweepResult :type "HitResult Structure (by ref)"))
  ;[1 1 1] Checking the for Player Character to trigger custom transition event
)

(event `/Game/LateShooter/MIscellaneous/BPI_Interactable.StartInteract`
  ;[1 1 1] door state triggers via interface
  (`self.TrasnitionToStates` (select `bool` false :`false` "NewEnumerator1" :`true` "NewEnumerator2" :!type "/Game/LateShooter/MIscellaneous/EDoorStates Enum")))

(event `/Game/LateShooter/MIscellaneous/BPI_Interactable.StopInteract`
  ;[1 1 1] door state triggers via interface
  (`self.TrasnitionToStates` "NewEnumerator0"))

(event `self.Box.OnComponentEndOverlap`
  (params (OverlappedComponent :type "PrimitiveComponent Object Reference") (OtherActor :type "Actor Object Reference") (OtherComp :type "PrimitiveComponent Object Reference") (OtherBodyIndex :type Integer))
  ;[1 1 1] Checking to See if Player is no longer overlapping Close Door
)

(event `TrasnitionToStates`
  (params (RequestedState :type "/Game/LateShooter/MIscellaneous/EDoorStates Enum" :default "NewEnumerator0"))
  ;[1 1 1] Custom Event to checking and updating door state and Animating with timeline
  (if (and (`|EnumInequality` RequestedState (`self.State`)) (not (`self.bTransitioning`)))
    (set `self.bStateQueued` false)
    (set `self.bTransitioning` true)
    (set `self.RequestedState` RequestedState)
    (bind (_direction _alpha) (`Timeline|TL_DoorOpening` :!via `PlayFromStart`)
      (:`Update`
        (`SceneComponent.K2_SetRelativeRotation` (`self.DoorMeshComp`) (`KismetMathLibrary.RLerp` (`BlueprintMapLibrary.Map_Find` (`self.TargetRotByEState`) (`self.State`)) (`BlueprintMapLibrary.Map_Find` (`self.TargetRotByEState`) (`self.RequestedState`)) _alpha) false false)
        (`KismetSystemLibrary.Delay` 5.0 :!label _label))
      (:`Finished`
        (set `self.State` (`self.RequestedState`))
        (set `self.bTransitioning` false)
        (if (`self.bStateQueued`)
          (`self.TrasnitionToStates` (`self.QueuedRequestState`))
          (goto _label))))
    (else
      (set `self.QueuedRequestState` RequestedState)
      (set `self.bStateQueued` true))))

(fn `UserConstructionScript`
  (`SceneComponent.K2_SetRelativeRotation` (`self.DoorMeshComp`) (`BlueprintMapLibrary.Map_Find` (`self.TargetRotByEState`) (`self.State`)) false false))