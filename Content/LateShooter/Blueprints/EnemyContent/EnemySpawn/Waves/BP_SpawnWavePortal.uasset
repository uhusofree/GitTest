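; Wave portal actor that spawns enemy AI at its WaveBox component's location.
; The LightWave event spawns one BP_Spooky per call, as long as the count of that class in the level stays under a fixed cap.
; HeavyWave is an empty event; similar capped spawn logic for BP_Enemy_Strong exists but is disconnected, so it never runs.
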(event `LightWave`
  (bind _outactors (`GameplayStatics.GetAllActorsOfClass` "/Game/LateShooter/Blueprints/EnemyContent/BP_Spooky.BP_Spooky_C"))
  (if (< (`KismetArrayLibrary.Array_Length` _outactors) 20)
    (`AIBlueprintHelperLibrary.SpawnAIFromClass` "/Game/LateShooter/Blueprints/EnemyContent/BP_Spooky.BP_Spooky_C" null (`SceneComponent.K2_GetComponentLocation` (`self.WaveBox`)))))

(event `HeavyWave`)

(fn `UserConstructionScript`)