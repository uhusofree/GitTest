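; BP_SpawnWavePortal2 is an enemy spawn portal that handles wave events by spawning AI at its WaveBox location.
; HeavyWave spawns one BP_Enemy_Strong per call, provided the world-wide count of that class is under a fixed cap.
; LightWave is empty, and a similar capped BP_Spooky spawn branch is left disconnected, so it never runs.
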(event `LightWave`)

(event `HeavyWave`
  (bind _outactors (`GameplayStatics.GetAllActorsOfClass` "/Game/LateShooter/Blueprints/EnemyContent/BP_Enemy_Strong.BP_Enemy_Strong_C"))
  (if (< (`KismetArrayLibrary.Array_Length` _outactors) 30)
    (`AIBlueprintHelperLibrary.SpawnAIFromClass` "/Game/LateShooter/Blueprints/EnemyContent/BP_Enemy_Strong.BP_Enemy_Strong_C" null (`SceneComponent.K2_GetComponentLocation` (`self.WaveBox`)))))

(fn `UserConstructionScript`)