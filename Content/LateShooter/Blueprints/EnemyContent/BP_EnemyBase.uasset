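; BP_EnemyBase is the base enemy Blueprint, killed by a single hit from a FirstPersonProjectile.
; A capsule hit spawns an explosion at the mesh, destroys the capsule and mesh components, and adds KillPoints to the kill tally in BP_GameState.
; It destroys only those components, not the actor, and the whole death sequence requires the BP_GameState cast to succeed.
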(event `self.CapsuleComponent.OnComponentHit`
  (params (HitComponent :type "PrimitiveComponent Object Reference") (OtherActor :type "Actor Object Reference") (OtherComp :type "PrimitiveComponent Object Reference") (NormalImpulse :type "Vector Structure") (Hit :type "HitResult Structure (by ref)"))
  (cast `/Game/LateShooter/Blueprints/FirstPersonProjectile` OtherActor)
  (bind _asbp_game_state (cast `/Game/LateShooter/MIscellaneous/BP_GameState` (`GameplayStatics.GetGameState`)))
  (`GameplayStatics.SpawnEmitterAtLocation` "/Game/StarterContent/Particles/P_Explosion.P_Explosion" (`SceneComponent.K2_GetComponentLocation` (`self.Mesh`)))
  (`ActorComponent.K2_DestroyComponent` (`self.CapsuleComponent`))
  (`ActorComponent.K2_DestroyComponent` (`self.Mesh`))
  (`/Game/LateShooter/MIscellaneous/BP_GameState.AddKills` _asbp_game_state (`self.KillPoints`)))

(fn `UserConstructionScript`)