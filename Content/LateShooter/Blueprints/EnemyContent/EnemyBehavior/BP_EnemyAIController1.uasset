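; BP_EnemyAIController1 is the enemy AI controller that runs the BT_Enemy behavior tree on possess.
; AI Perception updates write a successfully sensed Player-tagged actor to the TargetPlyr blackboard key.
; Any other perception update, whether a lost player or an untagged actor, clears that key.
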(event `self.ReceivePossess`
  (params (PossessedPawn :type "Pawn Object Reference"))
  (`self.RunBehaviorTree` "/Game/LateShooter/Blueprints/EnemyContent/EnemyBehavior/BT_Enemy.BT_Enemy"))

(event `self.AIPerception.OnTargetPerceptionUpdated`
  (params (Actor :type "Actor Object Reference") (Stimulus :type "AIStimulus Structure"))
  (if (and (`self.ActorHasTag` Actor "Player") (`.bSuccessfullySensed` (break `AIStimulus` Stimulus)))
    (`BlackboardComponent.SetValueAsObject` (`self.Blackboard`) "TargetPlyr" Actor)
    (else
      (`BlackboardComponent.SetValueAsObject` (`self.Blackboard`) "TargetPlyr" null))))

(fn `UserConstructionScript`)