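; Game state for the shooter that tracks score, kills and player health and decides when the match is won or lost.
; AddScore, AddKills and PlayerHealth update their values and compare them to thresholds on BP_GameMode, calling WinState or LoseState.
; Both states show a WBP_EndState widget with the matching result, enable the mouse cursor and pause the game.
; Delayed QuitGame nodes are left unconnected.
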(event `WinState`
  (bind _asplayer_controller (cast `PlayerController` (`GameplayStatics.GetPlayerController` 0)))
  (bind _returnvalue (`|CreateWidget` "/Game/LateShooter/MIscellaneous/WBP_EndState.WBP_EndState_C"))
  (set `/Game/LateShooter/MIscellaneous/WBP_EndState.EndState` "NewEnumerator1" _returnvalue)
  (`UserWidget.AddToViewport` _returnvalue 0)
  (set `PlayerController.bShowMouseCursor` true _asplayer_controller)
  (`GameplayStatics.SetGamePaused` true))

(event `LoseState`
  (bind _asplayer_controller (cast `PlayerController` (`GameplayStatics.GetPlayerController` 0)))
  (bind _returnvalue (`|CreateWidget` "/Game/LateShooter/MIscellaneous/WBP_EndState.WBP_EndState_C"))
  (set `/Game/LateShooter/MIscellaneous/WBP_EndState.EndState` "NewEnumerator0" _returnvalue)
  (`UserWidget.AddToViewport` _returnvalue 0)
  (set `PlayerController.bShowMouseCursor` true _asplayer_controller)
  (`GameplayStatics.SetGamePaused` true))

(fn `AddKills`
  (params (KillCount :type Integer :default 1))
  (returns (Kills :type Integer))
  (set `self.Kills` (+ KillCount (`self.Kills`)))
  (bind _asbp_game_mode (cast `/Game/LateShooter/MIscellaneous/BP_GameMode` (`GameplayStatics.GetGameMode`))
    (:`then`
      (if (>= (`self.Kills`) (`/Game/LateShooter/MIscellaneous/BP_GameMode.TargetKillGoal` _asbp_game_mode))
        (`self.WinState`)
        (return (`self.Kills`))
        (else
          (return (`self.Kills`)))))
    (:`CastFailed`
      (return (`self.Kills`)))))

(fn `AddScore`
  (params (PointsToAdd :type Integer :default 1))
  (returns (Score :type Integer))
  (set `self.Score` (+ PointsToAdd (`self.Score`)))
  (bind _asbp_game_mode (cast `/Game/LateShooter/MIscellaneous/BP_GameMode` (`GameplayStatics.GetGameMode`))
    (:`then`
      (if (>= (`self.Score`) (`/Game/LateShooter/MIscellaneous/BP_GameMode.ScoreToWin` _asbp_game_mode))
        (`self.WinState`)
        (return (`self.Score`))
        (else
          (return (`self.Score`)))))
    (:`CastFailed`
      (return (`self.Score`)))))

(fn `Player Health`
  (params (DamagedHealth :type "Float (double-precision)"))
  (returns (Health :type "Float (double-precision)"))
  (set `self.Health` DamagedHealth)
  (bind _asbp_game_mode (cast `/Game/LateShooter/MIscellaneous/BP_GameMode` (`GameplayStatics.GetGameMode`)))
  (if (<= (`self.Health`) (`/Game/LateShooter/MIscellaneous/BP_GameMode.PlayerCurrentHealth` _asbp_game_mode))
    (`self.LoseState`)
    (return (`self.Health`))))

(fn `UserConstructionScript`)